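; Player controller for mouse picking, apparently an early prototype for a chess game given its unconnected "White Chess Piece" tag check.
; On BeginPlay it shows the mouse cursor and calls SetViewTargetWithBlend with no target specified.
; A left click deprojects the cursor and starts a persistently drawn Visibility trace there, with no End point set.
; The debug prints for ray direction and hit actor tag never run, so clicks select nothing yet.
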(event EventBeginPlay
  (Game|Player|SetViewTargetwithBlend 0 0.0 "VTBlend_Linear" 0.0 false)
  (Variables|Default|SetbShowMouseCursor true))

(event EventTick
  (params (DeltaSeconds :type Float%20%28single-precision%29)))

(event Input|MouseEvents|LeftMouseButton
  (params (Key :type Key%20Structure :default "None"))
  (:Pressed
    (bind _returnvalue (Class|WidgetLayoutLibrary|GetMousePositiononViewport))
    (bind _outhit (Collision|LineTraceByChannel (.WorldPosition (Class|GameplayStatics|DeprojectScreentoWorld 0 _returnvalue)) "0, 0, 0" "TraceTypeQuery1" false 0 "Persistent"))))

(fn ConstructionScript)